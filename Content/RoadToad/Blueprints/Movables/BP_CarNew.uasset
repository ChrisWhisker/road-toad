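; BP_CarNew is a movable car obstacle in Road Toad that gets a random hue on each respawn through a shared dynamic material.
; Each car randomizes headlight tint, horn sound and pitch at BeginPlay.
; A toad entering HonkTrigger fires a rate-limited honk, pitched down when slowed, plus a roof-scale Timeline and brighter headlights in night mode.
; Parent event overrides toggle component collision and visibility and manage slow-mo and bubble power-ups.
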(event OnComponentBeginOverlap(HonkTrigger)
  (params (OverlappedComponent :type Primitive%20Component%20Object%20Reference) (OtherActor :type Actor%20Object%20Reference) (OtherComp :type Primitive%20Component%20Object%20Reference) (OtherBodyIndex :type Integer) (bFromSweep :type Boolean) (SweepResult :type Hit%20Result%20Structure%20%28by%20ref%29))
  (bind _returnvalue (Math|Float|MakeLiteralFloat 5e+03))
  (bind _returnvalue_2 (Math|Float|MakeLiteralFloat 1.5e+04))
  ;[1 0 0] car
  (Utilities|Casting|CastToBP_ThirdPersonToad OtherActor)
  (Utilities|FlowControl|DoOnce false :!label _label
    (:Completed
      (CallFunction|PlaySoundonComponent (Variables|Default|GetHonkAudio) 1.0 0 (* (select (Variables|Default|GetSlowed) 0.5 1.0) (Variables|Default|GetHornPitch)))
      (Utilities|FlowControl|Sequence
        (:then_0
          (Utilities|FlowControl|Delay 1.0)
          (goto _label Reset))
        (:then_1
          (if (Variables|/Game/RoadToad/Blueprints/BP_RoadToadGameMode.BP_RoadToadGameMode_C|GetNightMode (.AsBP%20Road%20Toad%20Game%20Mode (Utilities|Casting|CastToBP_RoadToadGameMode (Variables|Default|GetRoadToadGameMode))))
            (Rendering|Components|Light|SetIntensity (Variables|Default|GetSpotLight) _returnvalue_2)
            (Rendering|Components|Light|SetIntensity (Variables|Default|GetSpotLight1) _returnvalue_2)
            (bind _scale (Timeline|Timeline PlayFromStart)
              (:Update
                (Transformation|SetRelativeScale3D (Variables|Default|GetRoof) (* _scale (Variables|Default|GetOrigRoofScale))))
              (:Finished
                (Rendering|Components|Light|SetIntensity (Variables|Default|GetSpotLight) _returnvalue)
                (Rendering|Components|Light|SetIntensity (Variables|Default|GetSpotLight1) _returnvalue)))
            (else
              (Timeline|Timeline PlayFromStart))))))))

(event Custom|Disable
  (|CallParentFunction)
  (Collision|SetCollisionEnabled (Variables|Default|GetHonkTrigger) "NoCollision")
  (Rendering|SetVisibility (Variables|Default|GetRoof) false false)
  (Variables|Default|SetEnabled false))

(event Custom|Enable
  (|CallParentFunction)
  (Collision|SetCollisionEnabled (Variables|Default|GetHonkTrigger) "QueryAndPhysics")
  (Rendering|SetVisibility (Variables|Default|GetRoof) true false)
  (Variables|Default|SetEnabled true))

(event EventBeginPlay
  ;[1 0 0] car
  (|CallParentFunction)
  (bind _returnvalue (Rendering|Material|CreateDynamicMaterialInstance (Utilities|Array|Get(acopy) (Rendering|Material|GetMaterials (Variables|Default|GetChassis))) "None" "None" :!class /Script/Engine.KismetMaterialLibrary))
  (bind _output_get (Variables|Default|SetDMI _returnvalue))
  (Rendering|Material|SetMaterial (Variables|Default|GetChassis) 0 _output_get)
  (Class|Car|Respawn)
  (Rendering|Components|Light|SetLightColor (Variables|Default|GetSpotLight) (select (Math|Random|RandomBool) "(R=1.000000,G=1.000000,B=0.333000,A=1.000000)" "(R=1.000000,G=1.000000,B=1.000000,A=1.000000)") true)
  (Variables|Default|SetHornPitch (Math|Random|RandomFloatinRange 0.75 1.25))
  (Audio|Components|Audio|SetSound (Variables|Default|GetHonkAudio) (select (Math|Random|RandomBool) "/Game/RoadToad/Sounds/SW_HonkHonk.SW_HonkHonk" "/Game/RoadToad/Sounds/SW_Honk.SW_Honk"))
  (Variables|Default|SetOrigRoofScale (Variables|/Script/Engine.SceneComponent|GetRelativeScale3D (Variables|Default|GetRoof))))

(event EventRespawn
  (|CallParentFunction)
  ;[1 0 0] car
  (Variables|Default|SetPaintColor (Math|Color|MakeColor 1.0 1.0 1.0))
  (Class|KismetMathLibrary|LinearColorSetRandomHue (Variables|Default|GetPaintColor))
  (Rendering|Material|SetVectorParameterValue (Variables|Default|GetDMI) "Color" (Variables|Default|GetPaintColor) :!class /Script/Engine.MaterialInstanceDynamic))

(event EventDespawnPowerUps
  (|CallParentFunction)
  (CallFunction|DespawnPowerUps (Utilities|Array|MakeArray (Variables|Default|GetPowerUp_SlowMo) (Variables|Default|GetPowerUp_Bubble))))

(event EventSpawnPowerUp
  (params (Bubble :type Boolean))
  (|CallParentFunction Bubble)
  (CallFunction|SpawnPowerUp Bubble (Variables|Default|GetPowerUp_SlowMo) (Variables|Default|GetPowerUp_Bubble)))

(fn ConstructionScript
  (|CallParentFunction))