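; BP_Bird is a movable bird in RoadToad that flies back and forth across the level along X.
; Tick moves it by Speed, while a Fly timeline layers height and roll motion on top.
; Beyond RespawnDistance, a DoOnce-guarded random delay moves it to a random BP_BirdSpawn, setting direction from that spawn's side.
; Enable and Disable toggle the mesh's visibility and collision.
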(event Custom|TriggerRestart
  (Utilities|FlowControl|DoOnce false :!label _label
    (:Completed
      (Utilities|FlowControl|Delay (Math|Random|RandomFloatinRange 1.0 3.0))
      (CallFunction|Restart)
      (goto _label Reset))))

(event Custom|Restart
  (Variables|Default|SetLatestSpawn (.OutItem (Utilities|Array|Random (Variables|Default|GetBirdSpawns))))
  (Transformation|SetActorLocationAndRotation (.location (Transformation|GetActorTransform (Variables|Default|GetLatestSpawn))) (.rotation (Transformation|GetActorTransform (Variables|Default|GetLatestSpawn))))
  (Variables|Default|SetSpeed (Math|Float|SelectFloat (Math|Float|Absolute(Float) (Variables|Default|GetSpeed)) (* (Math|Float|Absolute(Float) (Variables|Default|GetSpeed)) -1.0) (< (.X (Math|Vector|BreakVector (.location (Transformation|GetActorTransform (Variables|Default|GetLatestSpawn))))) 0.0)))
  (if (Class|SourceControlHelpers|IsEnabled)
    (CallFunction|Enable)))

(event EventBeginPlay
  (bind _returnvalue (Transformation|GetActorLocation))
  (bind _returnvalue_2 (Transformation|GetActorRotation))
  (|CallParentFunction)
  (bind _outactors (Actor|GetAllActorsOfClass "/Game/RoadToad/Blueprints/BP_BirdSpawn.BP_BirdSpawn_C"))
  (Variables|Default|SetBirdSpawns _outactors)
  (bind (_direction _height _roll) (Timeline|Fly Play)
    (:Update
      (Transformation|SetActorLocationAndRotation (Math|Vector|MakeVector (.x _returnvalue) (.y _returnvalue) (+ (.z _returnvalue) _height)) (Math|Rotator|MakeRotator _roll (.pitch _returnvalue_2) (.yaw _returnvalue_2))))))

(event EventTick
  (params (DeltaSeconds :type Float%20%28single-precision%29))
  (bind _returnvalue (Transformation|GetActorLocation))
  (bind _respawndistance (Variables|Default|GetRespawnDistance))
  (if (and (< (.x _returnvalue) _respawndistance) (> (.x _returnvalue) (* _respawndistance -1.0))) ; if within level
    (Transformation|SetActorLocation (Math|Vector|MakeVector (+ (* DeltaSeconds (Variables|Default|GetSpeed)) (.x _returnvalue)) (.y _returnvalue) (.z _returnvalue)) false false)
    (else
      (CallFunction|TriggerRestart))))

(event EventEnable
  (bind _staticmesh (Variables|Default|GetStaticMesh))
  (|CallParentFunction)
  (Collision|SetCollisionEnabled _staticmesh "QueryAndPhysics")
  (Rendering|SetVisibility _staticmesh true false)
  (Variables|Default|SetEnabled true))

(event EventDisable
  (bind _staticmesh (Variables|Default|GetStaticMesh))
  (|CallParentFunction)
  (Collision|SetCollisionEnabled _staticmesh "NoCollision")
  (Rendering|SetVisibility _staticmesh false false)
  (Variables|Default|SetEnabled false))

(fn ConstructionScript
  (|CallParentFunction))