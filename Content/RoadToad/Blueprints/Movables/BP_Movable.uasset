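; BP_Movable is a RoadToad actor that slides along world X at a set Speed and loops between both ends of its travel range.
; While Enabled, Tick moves it without sweep, scaled by delta time.
; Passing RespawnDistance on either side teleports it to the opposite edge, then calls Respawn, an empty event here.
; BeginPlay caches the RoadToad game mode, though the movement logic does not use it.
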(event Custom|Respawn)

(event EventTick
  (params (DeltaSeconds :type Float%20%28single-precision%29))
  (bind _returnvalue (Transformation|GetActorLocation))
  (bind _respawndistance (Variables|Default|GetRespawnDistance))
  (bind _returnvalue_2 (* _respawndistance -1.0))
  (if (Variables|Default|GetEnabled)
    (if (> (.x _returnvalue) (Variables|Default|GetRespawnDistance))
      (Transformation|SetActorLocation (Math|Vector|MakeVector _returnvalue_2 (.y _returnvalue) (.z _returnvalue)) false true)
      (CallFunction|Respawn)
      (elif (< (.x _returnvalue) _returnvalue_2)
        (Transformation|SetActorLocation (Math|Vector|MakeVector (Variables|Default|GetRespawnDistance) (.y _returnvalue) (.z _returnvalue)) false true)
        (CallFunction|Respawn)
        (else
          (Transformation|SetActorLocation (Math|Vector|MakeVector (+ (* DeltaSeconds (Variables|Default|GetSpeed)) (.x _returnvalue)) (.y _returnvalue) (.z _returnvalue)) false false))))))

(event EventBeginPlay
  (|CallParentFunction)
  (bind _asbp_road_toad_game_mode (Utilities|Casting|CastToBP_RoadToadGameMode (Game|GetGameMode)))
  (Variables|Default|SetRoadToadGameMode _asbp_road_toad_game_mode))

(fn ConstructionScript)