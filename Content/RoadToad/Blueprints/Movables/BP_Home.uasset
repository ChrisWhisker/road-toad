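; BP_Home is a lily pad home in Road Toad that can be closed with a toad on it or opened again.
; CloseHome enables the blocking box collision and shows the toad mesh, while OpenHome reverses both.
; The construction script starts the box with no collision, and BeginPlay gives the lily pad a random yaw after calling the parent.
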(event Custom|CloseHome
  (Collision|SetCollisionEnabled (Variables|Default|GetBlockingBox) "QueryAndPhysics")
  (Rendering|SetVisibility (Variables|Default|GetStaticMesh_Toad) true false))

(event Custom|OpenHome
  (Collision|SetCollisionEnabled (Variables|Default|GetBlockingBox) "NoCollision")
  (Rendering|SetVisibility (Variables|Default|GetStaticMesh_Toad) false false))

(event EventBeginPlay
  (|CallParentFunction)
  (Transformation|SetRelativeRotation (Variables|Default|GetStaticMesh_LilyPad) (Math|Rotator|MakeRotator 0.0 0.0 (Math|Random|RandomFloatinRange 0.0 3.6e+02)) false false))

(fn ConstructionScript
  (Collision|SetCollisionEnabled (Variables|Default|GetBlockingBox) "NoCollision"))