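; Movable chain of three turtle shells that swim and sometimes dive, with slow-mo and bubble power-up spawn hooks.
; A Swim timeline animates the shells' sideways position and yaw.
; Respawn resets height and rotation, randomizes shell colors through dynamic materials, then after a random delay may start the Dive timeline.
; Dive offsets actor height from its initial value, tilts the shells and plays a splash on entering water.
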(event EventBeginPlay
  (bind _sm_turtleshell2 (Variables|Default|GetSM_TurtleShell2))
  (bind _sm_turtleshell1 (Variables|Default|GetSM_TurtleShell1))
  (bind _sm_turtleshell1_2 (Variables|Default|GetSM_TurtleShell1))
  (bind _sm_turtleshell (Variables|Default|GetSM_TurtleShell))
  (bind _sm_turtleshell2_2 (Variables|Default|GetSM_TurtleShell2))
  (bind _sm_turtleshell_2 (Variables|Default|GetSM_TurtleShell))
  (bind _relativerotation (Variables|/Script/Engine.SceneComponent|GetRelativeRotation _sm_turtleshell2_2))
  (bind _relativelocation (Variables|/Script/Engine.SceneComponent|GetRelativeLocation _sm_turtleshell))
  (bind _relativelocation_2 (Variables|/Script/Engine.SceneComponent|GetRelativeLocation _sm_turtleshell1_2))
  (bind _relativelocation_3 (Variables|/Script/Engine.SceneComponent|GetRelativeLocation _sm_turtleshell2_2))
  (|CallParentFunction)
  (bind _returnvalue (Rendering|Material|CreateDynamicMaterialInstance (Utilities|Array|Get(acopy) (Rendering|Material|GetMaterials _sm_turtleshell_2)) "None" "None" :!class /Script/Engine.KismetMaterialLibrary))
  (bind _output_get (Variables|Default|SetDMI_Shell1 _returnvalue))
  (Rendering|Material|SetMaterial _sm_turtleshell_2 0 _output_get)
  (bind _returnvalue_2 (Rendering|Material|CreateDynamicMaterialInstance (Utilities|Array|Get(acopy) (Rendering|Material|GetMaterials _sm_turtleshell1)) "None" "None" :!class /Script/Engine.KismetMaterialLibrary))
  (bind _output_get_2 (Variables|Default|SetDMI_Shell2 _returnvalue_2))
  (Rendering|Material|SetMaterial _sm_turtleshell1 0 _output_get_2)
  (bind _returnvalue_3 (Rendering|Material|CreateDynamicMaterialInstance (Utilities|Array|Get(acopy) (Rendering|Material|GetMaterials _sm_turtleshell2)) "None" "None" :!class /Script/Engine.KismetMaterialLibrary))
  (bind _output_get_3 (Variables|Default|SetDMI_Shell3 _returnvalue_3))
  (Rendering|Material|SetMaterial _sm_turtleshell2 0 _output_get_3)
  (Variables|Default|SetInitialHeight (.z (Transformation|GetActorLocation)))
  (Class|TurtleChain|Respawn)
  (bind (_direction _horizontalposition _rotation) (Timeline|Swim Play)
    (:Update
      (Transformation|SetRelativeLocation _sm_turtleshell (Math|Vector|MakeVector (.x _relativelocation) _horizontalposition (.z _relativelocation)) false false)
      (Transformation|SetRelativeLocation _sm_turtleshell1_2 (Math|Vector|MakeVector (.x _relativelocation_2) _horizontalposition (.z _relativelocation_2)) false false)
      (Transformation|SetRelativeLocation _sm_turtleshell2_2 (Math|Vector|MakeVector (.x _relativelocation_3) _horizontalposition (.z _relativelocation_3)) false false)
      (Transformation|SetRelativeRotation (Variables|Default|GetSM_TurtleShell) (Math|Rotator|MakeRotator (.roll _relativerotation) (.pitch _relativerotation) _rotation) false false))))

(event EventDespawnPowerUps
  ;[1 1 1] todo move this to C++ so it's not copied in each BP movable class
  (CallFunction|DespawnPowerUps (Utilities|Array|MakeArray (Variables|Default|GetPowerUp_SlowMo) (Variables|Default|GetPowerup_Bubble))))

(event EventSpawnPowerUp
  (params (Bubble :type Boolean))
  ;[1 1 1] todo move this to C++ so it's not copied in each BP movable class
  (CallFunction|SpawnPowerUp Bubble (Variables|Default|GetPowerUp_SlowMo) (Variables|Default|GetPowerup_Bubble)))

(event EventRespawn
  (bind _returnvalue (Transformation|GetActorLocation))
  (bind _returnvalue_2 (Transformation|GetActorLocation))
  (bind _sm_turtleshell (Variables|Default|GetSM_TurtleShell))
  (bind _relativerotation (Variables|/Script/Engine.SceneComponent|GetRelativeRotation _sm_turtleshell))
  (Utilities|FlowControl|Sequence
    (:then_0
      (bind (_direction _height _tilt) (Timeline|Dive Stop)
        (:Update
          (Transformation|SetActorLocation (Math|Vector|MakeVector (.x _returnvalue) (.y _returnvalue) (+ _height (Variables|Default|GetInitialHeight))) false false)
          (Transformation|SetRelativeRotation _sm_turtleshell (Math|Rotator|MakeRotator (.roll _relativerotation) _tilt (.yaw _relativerotation)) false false))
        (:OnEnterWater
          (CallFunction|PlaySoundonComponent (Variables|Default|GetSplashAudio) 1.0 "/Game/RoadToad/Sounds/SW_Splash.SW_Splash" 0.0))))
    (:then_1
      (Transformation|SetActorLocation (Math|Vector|MakeVector (.x _returnvalue_2) (.y _returnvalue_2) (Variables|Default|GetInitialHeight)) false false)
      (Transformation|SetRelativeRotation (Variables|Default|GetSM_TurtleShell) (Math|Rotator|MakeRotator 0.0 0.0 0.0) false false))
    (:then_2
      (Rendering|Material|SetVectorParameterValue (Variables|Default|GetDMI_Shell1) "Color" (Utilities|RandomShellColor) :!class /Script/Engine.MaterialInstanceDynamic)
      (Rendering|Material|SetVectorParameterValue (Variables|Default|GetDMI_Shell2) "Color" (Utilities|RandomShellColor) :!class /Script/Engine.MaterialInstanceDynamic)
      (Rendering|Material|SetVectorParameterValue (Variables|Default|GetDMI_Shell3) "Color" (Utilities|RandomShellColor) :!class /Script/Engine.MaterialInstanceDynamic)
      (Utilities|FlowControl|Delay (Math|Random|RandomFloatinRange 0.0 1.0))
      (if (Math|Random|RandomBool)
        (Timeline|Dive Play)))))

(fn ConstructionScript
  (|CallParentFunction))