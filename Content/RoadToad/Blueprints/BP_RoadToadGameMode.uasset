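; Game mode for Road Toad, a Frogger-style game, running the toad's life cycle, level flow and UI.
; Deaths are gated, switch to an outcome camera and slow time before respawning a fresh pawn at a random PlayerStart or waiting for retry.
; Filling five homes completes a level; the next speeds up all cached cars, logs and turtle chains.
; Power-up events slow movers and fade lighting into night with car headlights via a timeline.
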(event Custom|ToadEnteredHome
  (params (Home :type BP%20Home%20Object%20Reference))
  ;[1 0 0] game flow
  (if (not (Utilities|Array|ContainsItem (Class|RoadToadGameState|GetOccupiedHomes (Variables|Default|GetRoadToadGameState)) Home))
    (CallFunction|ProhibitDeath)
    (Class|TimerSubsystem|PauseLifeTimer (Subsystems|GetTimerSubsystem))
    (Class|AudioSubsystem|PlaySound (Subsystems|GetAudioSubsystem) "/Game/RoadToad/Sounds/SW_Ribbit.SW_Ribbit" 1.0)
    (CallFunction|SwitchtoOutcomeCamera)
    (Class|RoadToadGameState|AddtoOccupiedHomes (Variables|Default|GetRoadToadGameState) (Utilities|ResolveSoftReference Home))
    (Rendering|SetActorHiddenInGame (Variables|Default|GetToadPawn) true)
    (CallFunction|SetIgnoreInput true)
    (Transformation|SetActorLocationAndRotation (Variables|Default|GetToadPawn) (Transformation|GetActorLocation Home) (Transformation|GetActorRotation Home) false true)
    (Class|ScoringSubsystem|AddPoints (Subsystems|GetScoringSubsystem) (+ (Math|Float|Round (* (Class|TimerSubsystem|GetLifeTimerSecondsLeft (Subsystems|GetTimerSubsystem)) 1e+01)) 50))
    (Default|CloseHome Home)
    (if (>= (Utilities|Array|Length (Class|RoadToadGameState|GetOccupiedHomes (Variables|Default|GetRoadToadGameState))) 5)
      (Class|RoadToadHUD|ShowLevelComplete (Variables|Default|GetRoadToadHUD) (Class|RoadToadGameState|GetCurrentLevel (Variables|Default|GetRoadToadGameState)))
      (Variables|Default|SetCanStartNextLevel true)
      (else
        (Utilities|FlowControl|Delay 1.0)
        (CallFunction|RespawnToad)))))

(event Custom|RespawnToad
  ;[0 1 0] toad life cycle
  (Class|TimerSubsystem|TickJumpTimer (Subsystems|GetTimerSubsystem) (Variables|Default|GetJumpTimerMaxSeconds))
  (bind _returnvalue (Game|SpawnActorfromClass "/Game/RoadToad/Blueprints/BP_ThirdPersonToad.BP_ThirdPersonToad_C" (Transformation|GetActorTransform (Class|GameModeBase|FindPlayerStart (Game|GetPlayerController 0))) "AlwaysSpawn" "MultiplyWithRoot" 0 0))
  (Actor|DestroyActor (Variables|Default|GetToadPawn))
  (bind _output_get (Variables|Default|SetToadPawn _returnvalue))
  (Pawn|Possess (Game|GetPlayerController 0) _output_get)
  (Rendering|SetActorHiddenInGame (Variables|Default|GetToadPawn) false)
  (Class|RoadToadHUD|HideDeathUI (Variables|Default|GetRoadToadHUD))
  (Variables|/Script/Engine.PostProcessVolume|SetSettings (Variables|Default|GetPostProcessVolume) (Utilities|Struct|MakePostProcessSettings (Math|Vector4|MakeVector4 1.0 1.0 1.0 1.0)))
  (Utilities|Time|SetGlobalTimeDilation 1.0)
  (Physics|SetSimulatePhysics (Variables|/Script/Engine.Character|GetCapsuleComponent (Variables|Default|GetToadPawn)) false)
  (CallFunction|SetIgnoreInput false)
  (Class|TimerSubsystem|RestartLifeTimer (Subsystems|GetTimerSubsystem))
  (CallFunction|AllowDeath)
  (Class|RoadToadHUD|ShowBottomPanel (Variables|Default|GetRoadToadHUD))
  (Default|RemoveBubble (Variables|Default|GetToadPawn))
  (CallFunction|ResetMovablesSpeed true)
  (Class|PowerUpSubsystem|DespawnPowerUps (Subsystems|GetPowerUpSubsystem)))

(event Custom|ToggleNightMode
  ;[1 0 1] Powerup (night mode)
  (bind _isa (Utilities|FlowControl|FlipFlop)
    (:A
      _)
    (:B
      _))
  (Variables|Default|SetNightMode _isa)
  (if (Variables|Default|GetNightMode)
    (bind _alpha (Timeline|FadeToNight PlayFromStart)
      (:Update
        (Rendering|Components|Light|SetLightColor (Variables|/Script/Engine.Light|GetLightComponent (Variables|Default|GetSunLight)) (Math|Color|Lerp(LinearColor) "(R=1.000000,G=1.000000,B=1.000000,A=1.000000)" (Variables|Default|GetNightLightColor) _alpha) true)
        (Rendering|Components|Light|SetIntensity (Variables|/Script/Engine.Light|GetLightComponent (Variables|Default|GetFrontalLight)) (- 1.0 _alpha)))
      (:Headlights
        (for _array_element (Variables|Default|GetCars)
          (if (Variables|/Script/RoadToad.Movable|GetEnabled _array_element)
            (Rendering|SetVisibility (Variables|/Game/RoadToad/Blueprints/Movables/BP_Car.BP_Car_C|GetSpotLight _array_element) (Variables|Default|GetNightMode) false)))))
    (else
      (Timeline|FadeToNight ReverseFromEnd))))

(event Custom|SlowMovables
  (bind _nightmode (Variables|Default|GetNightMode))
  ;[1 0 1] Powerup (slowmo)
  (Variables|Default|SetWasNightModeBeforeSlow _nightmode)
  (if _nightmode
    _
    (else
      (CallFunction|SwitchtoNight)))
  (for _array_element (Variables|Default|GetMovables)
    (if (Variables|/Script/RoadToad.Movable|GetEnabled _array_element)
      (if (not (Variables|/Script/RoadToad.Movable|GetSlowed _array_element))
        (Variables|/Script/RoadToad.Movable|SetSpeed _array_element (/ (Variables|/Script/RoadToad.Movable|GetSpeed _array_element) (Variables|Default|GetMovableSlowingFactor)))
        (Variables|/Script/RoadToad.Movable|SetSlowed _array_element true))))
  (Audio|Components|Audio|SetPitchMultiplier (Variables|/Script/Engine.AmbientSound|GetAudioComponent (Variables|Default|GetMusicActor)) 0.5)
  (Utilities|FlowControl|Delay 5.0)
  (CallFunction|ResetMovablesSpeed false)
  (Class|PowerUpSubsystem|TriggerSpawnPowerUp (Subsystems|GetPowerUpSubsystem)))

(event Custom|ResetMovablesSpeed
  (params (CalledByRespawn :type Boolean))
  ;[1 0 1] Powerup (slowmo)
  (if CalledByRespawn
    _
    (elif (Variables|Default|GetWasNightModeBeforeSlow)
      _
      (else
        (CallFunction|SwitchtoDay))))
  (for _array_element (Variables|Default|GetMovables)
    (if (Variables|/Script/RoadToad.Movable|GetEnabled _array_element)
      (if (Variables|/Script/RoadToad.Movable|GetSlowed _array_element)
        (Variables|/Script/RoadToad.Movable|SetSpeed _array_element (* (Variables|/Script/RoadToad.Movable|GetSpeed _array_element) (Variables|Default|GetMovableSlowingFactor)))
        (Variables|/Script/RoadToad.Movable|SetSlowed _array_element false))))
  (Audio|Components|Audio|SetPitchMultiplier (Variables|/Script/Engine.AmbientSound|GetAudioComponent (Variables|Default|GetMusicActor)) 1.0))

(event Custom|TryStartNextLevel
  ;[1 0 0] game flow
  (if (Variables|Default|GetCanStartNextLevel)
    (Variables|Default|SetCanStartNextLevel false)
    (Class|RoadToadHUD|HideLevelComplete (Variables|Default|GetRoadToadHUD))
    (bind _returnvalue (Class|RoadToadGameState|IncrementLevel (Variables|Default|GetRoadToadGameState)))
    (Class|RoadToadHUD|UpdateLevelNumber (Variables|Default|GetRoadToadHUD) _returnvalue)
    (Class|ScoringSubsystem|UpdateScoreMultiplier (Subsystems|GetScoringSubsystem) _returnvalue)
    (for _array_element (Variables|Default|GetMovables)
      (Variables|/Script/RoadToad.Movable|SetSpeed _array_element (* (Variables|/Script/RoadToad.Movable|GetSpeed _array_element) 1.25)))
    (Variables|Default|SetCanRestart true)
    (CallFunction|TryRestart false)))

(event Custom|ToadMadeFirstMove
  ;[1 0 0] game flow
  (Class|PowerUpSubsystem|TriggerSpawnPowerUp (Subsystems|GetPowerUpSubsystem))
  (Class|TimerSubsystem|RestartLifeTimer (Subsystems|GetTimerSubsystem)))

(event Custom|SwitchToDay
  ;[1 0 1] Powerup (night mode)
  (Variables|Default|SetNightMode false)
  (if (Variables|Default|GetNightMode)
    (bind _alpha (Timeline|FadeToNight PlayFromStart)
      (:Update
        (Rendering|Components|Light|SetLightColor (Variables|/Script/Engine.Light|GetLightComponent (Variables|Default|GetSunLight)) (Math|Color|Lerp(LinearColor) "(R=1.000000,G=1.000000,B=1.000000,A=1.000000)" (Variables|Default|GetNightLightColor) _alpha) true)
        (Rendering|Components|Light|SetIntensity (Variables|/Script/Engine.Light|GetLightComponent (Variables|Default|GetFrontalLight)) (- 1.0 _alpha)))
      (:Headlights
        (for _array_element (Variables|Default|GetCars)
          (if (Variables|/Script/RoadToad.Movable|GetEnabled _array_element)
            (Rendering|SetVisibility (Variables|/Game/RoadToad/Blueprints/Movables/BP_Car.BP_Car_C|GetSpotLight _array_element) (Variables|Default|GetNightMode) false)))))
    (else
      (Timeline|FadeToNight ReverseFromEnd))))

(event Custom|SwitchToNight
  ;[1 0 1] Powerup (night mode)
  (Variables|Default|SetNightMode true)
  (if (Variables|Default|GetNightMode)
    (bind _alpha (Timeline|FadeToNight PlayFromStart)
      (:Update
        (Rendering|Components|Light|SetLightColor (Variables|/Script/Engine.Light|GetLightComponent (Variables|Default|GetSunLight)) (Math|Color|Lerp(LinearColor) "(R=1.000000,G=1.000000,B=1.000000,A=1.000000)" (Variables|Default|GetNightLightColor) _alpha) true)
        (Rendering|Components|Light|SetIntensity (Variables|/Script/Engine.Light|GetLightComponent (Variables|Default|GetFrontalLight)) (- 1.0 _alpha)))
      (:Headlights
        (for _array_element (Variables|Default|GetCars)
          (if (Variables|/Script/RoadToad.Movable|GetEnabled _array_element)
            (Rendering|SetVisibility (Variables|/Game/RoadToad/Blueprints/Movables/BP_Car.BP_Car_C|GetSpotLight _array_element) (Variables|Default|GetNightMode) false)))))
    (else
      (Timeline|FadeToNight ReverseFromEnd))))

(event Custom|ShowHUD
  ;[1 1 1] UI
  (Class|RootWidget|ShowHUD (Variables|Default|GetRootWidget)))

(event Custom|Pause
  ;[1 1 1] UI
  (Game|SetGamePaused true)
  (Class|RootWidget|ShowPauseMenu (Variables|Default|GetRootWidget)))

(event Custom|RetryReady
  ;[0 1 0] toad life cycle
  (EventDispatchers|UnbindEventfromRetryReady (Variables|Default|GetRoadToadHUD) (delegate Custom|RetryReady))
  (Variables|Default|SetCanRestart true))

(event Custom|SwitchToOutcomeCamera
  (Utilities|IsValid (Variables|Default|GetOutcomeCam)
    (:Is%20Valid
      _)
    (:Is%20Not%20Valid
      (bind _outactors (Actor|GetAllActorsOfClasswithTag "/Script/Engine.CameraActor" "Outcome"))
      (Variables|Default|SetOutcomeCam (Utilities|Array|Get(acopy) _outactors))))
  (bind _desiredview (Class|CameraComponent|GetCameraView (Variables|/Game/RoadToad/Blueprints/BP_ThirdPersonToad.BP_ThirdPersonToad_C|GetFollowCamera (Variables|Default|GetToadPawn)) 0.0))
  (Transformation|SetActorLocationAndRotation (Variables|Default|GetOutcomeCam) (.Location (Utilities|Struct|BreakMinimalViewInfo _desiredview)) (Math|Rotator|FindLookatRotation (.Location (Utilities|Struct|BreakMinimalViewInfo _desiredview)) (Transformation|GetActorLocation (Pawn|GetControlledPawn (Game|GetPlayerController 0)))))
  (Game|Player|SetViewTargetwithBlend (Game|GetPlayerController 0) (Variables|Default|GetOutcomeCam) 0.0 "VTBlend_Linear" 0.0 false))

(event Custom|SetIgnoreInput
  (params (NewIgnore :type Boolean))
  (bind _returnvalue (Game|GetPlayerController 0))
  (Input|SetIgnoreMoveInput _returnvalue NewIgnore)
  (Input|SetIgnoreLookInput _returnvalue NewIgnore))

(event Custom|NextLevel
  ;[1 0 0] game flow
  (Class|RoadToadHUD|ShowLevelComplete (Variables|Default|GetRoadToadHUD) (Class|RoadToadGameState|GetCurrentLevel (Variables|Default|GetRoadToadGameState)))
  (Variables|Default|SetCanStartNextLevel true))

(event Custom|OpenExitGameMenu
  ;[1 1 1] UI
  (Default|ShowExitGameMenu (Variables|Default|GetRootWidget)))

(event Custom|ProhibitDeath
  (bind _toadpawn (Variables|Default|GetToadPawn))
  ;[0 1 0] toad life cycle
  (Utilities|FlowControl|Gate false) ; enters at Close
)

(event Custom|AllowDeath
  (bind _toadpawn (Variables|Default|GetToadPawn))
  ;[0 1 0] toad life cycle
  (Utilities|FlowControl|Gate false) ; enters at Open
)

(event Custom|TryRestart
  (params (ResetScore :type Boolean))
  (bind _roadtoadgamestate (Variables|Default|GetRoadToadGameState))
  ;[1 0 0] game flow
  (if (Variables|Default|GetCanRestart)
    (Variables|Default|SetCanRestart false)
    (if ResetScore
      (Class|RoadToadGameState|ClearScore (Variables|Default|GetRoadToadGameState))
      (Class|RoadToadHUD|UpdateScore (Variables|/Game/RoadToad/Blueprints/Widgets/WBP_Root.WBP_Root_C|GetHUD (Variables|Default|GetRootWidget))))
    (Class|RoadToadGameState|EmptyOccupiedHomes _roadtoadgamestate)
    (Class|RoadToadGameState|ResetLives _roadtoadgamestate)
    (Class|RoadToadHUD|ResetUI (Variables|Default|GetRoadToadHUD))
    (for _array_element (Variables|Default|GetToadHomes)
      (Default|OpenHome _array_element))
    (for _array_element_2 (Variables|Default|GetCars)
      (if (not (Variables|/Script/RoadToad.Movable|GetEnabled _array_element_2))
        (Default|Enable _array_element_2)))
    (CallFunction|RespawnToad)))

(event EventBeginPlay
  (bind _returnvalue (UserInterface|CreateWidget "/Game/RoadToad/Blueprints/Widgets/WBP_Root.WBP_Root_C"))
  (bind _output_get (Variables|Default|SetRootWidget _returnvalue))
  (UserInterface|Viewport|AddtoViewport _output_get 0)
  (Class|RootWidget|ShowPauseMenu (Variables|Default|GetRootWidget))
  (Class|RootWidget|HideHUD (Variables|Default|GetRootWidget))
  (Class|Actor|SetTickablewhenPaused true)
  (Variables|Default|SetRoadToadHUD (Utilities|ResolveSoftReference (Class|RootWidget|GetHUD (Variables|Default|GetRootWidget))))
  (bind _outactors (Actor|GetAllActorsOfClasswithTag "/Script/Engine.CameraActor" "Startup"))
  (Game|Player|SetViewTargetwithBlend (Game|GetPlayerController 0) (Utilities|Array|Get(acopy) _outactors) 0.0 "VTBlend_Linear" 0.0 false)
  (bind _outactors_2 (Actor|GetAllActorsOfClasswithTag "/Script/Engine.DirectionalLight" "sun"))
  (Variables|Default|SetSunLight (Utilities|Array|Get(acopy) _outactors_2))
  (CallFunction|SetIgnoreInput true)
  (Variables|/Script/Engine.PlayerController|SetbShowMouseCursor (Game|GetPlayerController 0) true)
  (bind _outactors_3 (Actor|GetAllActorsOfClasswithTag "/Script/Engine.DirectionalLight" "front"))
  (Variables|Default|SetFrontalLight (Utilities|Array|Get(acopy) _outactors_3))
  (bind _returnvalue_2 (Actor|GetActorOfClass "/Script/Engine.PostProcessVolume"))
  (Variables|Default|SetPostProcessVolume _returnvalue_2)
  (bind _asroad_toad_game_state (Utilities|Casting|CastToRoadToadGameState (Game|GetGameState)))
  (Variables|Default|SetRoadToadGameState _asroad_toad_game_state)
  (bind _asbp_third_person_toad (Utilities|Casting|CastToBP_ThirdPersonToad (Game|Player|GetPlayerPawn 0)))
  (Variables|Default|SetToadPawn _asbp_third_person_toad)
  (bind _outactors_4 (Actor|GetAllActorsOfClass "/Game/RoadToad/Blueprints/BP_Home.BP_Home_C"))
  (Variables|Default|SetToadHomes _outactors_4)
  (bind _outactors_5 (Actor|GetAllActorsOfClass "/Script/RoadToad.Movable"))
  (bind _output_get_2 (Variables|Default|SetMovables _outactors_5))
  (for _array_element _output_get_2
    (bind _asbp_car (Utilities|Casting|CastToBP_Car _array_element)
      (:then
        (Utilities|Array|Add (Variables|Default|GetCars) _asbp_car))
      (:CastFailed
        (bind _asbp_log (Utilities|Casting|CastToBP_Log _array_element)
          (:then
            (Utilities|Array|Add (Variables|Default|GetLogs) _asbp_log))
          (:CastFailed
            (bind _asbp_turtle_chain (Utilities|Casting|CastToBP_TurtleChain _array_element))
            (Utilities|Array|Add (Variables|Default|GetTurtleChains) _asbp_turtle_chain))))))
  (bind _returnvalue_3 (Actor|GetActorOfClass "/Script/Engine.AmbientSound"))
  (Variables|Default|SetMusicActor _returnvalue_3))

(event EventKillToad
  (params (CauseOfDeath :type ECauseOfDeath%20Enum :default "Car"))
  (bind _toadpawn (Variables|Default|GetToadPawn))
  ;[0 1 0] toad life cycle
  (Utilities|FlowControl|Gate false
    (:Exit
      (CallFunction|SwitchtoOutcomeCamera)
      (Class|AudioSubsystem|PlaySound (Subsystems|GetAudioSubsystem) (Utilities|Select :Index CauseOfDeath :Car "/Game/RoadToad/Sounds/SW_Splat.SW_Splat" :Water "/Game/RoadToad/Sounds/SW_Splash.SW_Splash" :Timer "/Game/RoadToad/Sounds/SW_Ribbit.SW_Ribbit") (Utilities|Select :Index CauseOfDeath :Car 1.0 :Water 1.0 :Timer 0.5))
      (CallFunction|ProhibitDeath)
      (if (Utilities|Enum|Equal(Enum) CauseOfDeath "Car")
        (Default|Flatten (Variables|Default|GetToadPawn)))
      (Class|TimerSubsystem|PauseLifeTimer (Subsystems|GetTimerSubsystem))
      (Class|RoadToadHUD|HideBottomPanel (Variables|Default|GetRoadToadHUD))
      (CallFunction|SetIgnoreInput true)
      (Variables|/Script/Engine.PostProcessVolume|SetSettings (Variables|Default|GetPostProcessVolume) (Utilities|Struct|MakePostProcessSettings (Math|Vector4|MakeVector4 0.5 0.5 0.5 0.5)))
      (Default|StopJumpAnimation _toadpawn)
      (Physics|SetSimulatePhysics (Variables|/Script/Engine.Character|GetCapsuleComponent _toadpawn) true)
      (bind _returnvalue (Class|RoadToadGameState|TakeALife (Variables|Default|GetRoadToadGameState)))
      (Class|RoadToadHUD|UpdateLivesLeft (Variables|Default|GetRoadToadHUD) _returnvalue)
      (Utilities|Time|SetGlobalTimeDilation 0.1)
      (if (>= _returnvalue 0)
        (Class|RoadToadHUD|ShowDeathUI (Variables|Default|GetRoadToadHUD) CauseOfDeath)
        (Utilities|FlowControl|Delay 0.15)
        (CallFunction|RespawnToad)
        (else
          (EventDispatchers|BindEventtoRetryReady (Variables|Default|GetRoadToadHUD) (delegate Custom|RetryReady)))))))

(fn ConstructionScript)

(fn FindPlayerStart
  (params (Player :type Controller%20Object%20Reference) (IncomingName :type String))
  (if (== (Utilities|Array|Length (Variables|Default|GetPlayerStarts)) 0)
    (bind _outactors (Actor|GetAllActorsOfClass "/Script/Engine.PlayerStart"))
    (Variables|Default|SetPlayerStarts _outactors))
  (return (Utilities|Array|Get(acopy) (Variables|Default|GetPlayerStarts) (Math|Random|RandomIntegerinRange 0 (Utilities|Array|LastIndex (Variables|Default|GetPlayerStarts))))))