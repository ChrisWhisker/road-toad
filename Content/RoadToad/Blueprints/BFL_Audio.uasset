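; BFL_Audio is a Road Toad Blueprint function library with a helper for playing sound on an existing audio component.
; PlaySoundOnComponent optionally swaps the sound and pitch, then plays the component at the audio subsystem's sounds volume scaled by a multiplier.
; It updates component volume only when the value differs, and prints a warning instead of playing when the multiplier is not positive.
; An invalid component is silently ignored, as its warning print is unreachable.
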(fn PlaySoundonComponent
  (params (AudioComponent :type Audio%20Component%20Object%20Reference) (VolumeMultiplier :type Float%20%28double-precision%29) (OptionalSound :type Sound%20Base%20Object%20Reference) (OptionalPitch :type Float%20%28double-precision%29))
  (bind _returnvalue (Subsystems|GetAudioSubsystem))
  (bind _returnvalue_2 (Class|AudioSubsystem|GetSoundsVolume _returnvalue))
  (bind _returnvalue_3 (* _returnvalue_2 VolumeMultiplier))
  (Utilities|IsValid AudioComponent
    (:Is%20Valid
      (if (> VolumeMultiplier 0.0)
        (Utilities|IsValid OptionalSound
          (:Is%20Valid
            (Audio|Components|Audio|SetSound AudioComponent OptionalSound))
          (:Is%20Not%20Valid
            _))
        (if (> OptionalPitch 0.0)
          (Audio|Components|Audio|SetPitchMultiplier AudioComponent OptionalPitch))
        (if (!= _returnvalue_3 (Variables|/Script/Engine.AudioComponent|GetVolumeMultiplier AudioComponent))
          (Audio|Components|Audio|SetVolumeMultiplier AudioComponent _returnvalue_3 :!class /Script/Engine.AudioComponent))
        (Audio|Components|Audio|Play AudioComponent 0.0)
        (else
          (Development|PrintString AudioComponent "Volume must be greater than 0." true true "(R=1.000000,G=0.000000,B=0.000000,A=1.000000)"))))))