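; Game mode for a Frogger-style toad game, running the life cycle, homes, scoring, timers, levels and pause menu.
; BeginPlay caches lights, HUD and movable cars, logs and turtle chains that later events drive.
; A gate blocks repeated deaths; death and home events switch to an outcome camera, then respawn a fresh pawn or await retry or next level.
; Powerups spawn by frog progress; slowmo slows movables and music under a timeline-faded night.
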(event Custom|FrogEnteredHome
  (params (Home :type BP%20Home%20Object%20Reference))
  ;[1 0 0] game flow
  (if (not (Utilities|Array|ContainsItem (Class|RoadToadGameState|GetOccupiedHomes (Variables|Default|GetRoadToadGameState)) Home))
    (CallFunction|ProhibitDeath)
    (CallFunction|StopTimer)
    (Class|AudioSubsystem|PlaySound (Subsystems|GetAudioSubsystem) "/Game/RoadToad/Sounds/SW_Ribbit.SW_Ribbit" 1.0)
    (CallFunction|SwitchtoOutcomeCamera)
    (Class|RoadToadGameState|AddtoOccupiedHomes (Variables|Default|GetRoadToadGameState) Home)
    (Rendering|SetActorHiddenInGame (Variables|Default|GetFrogPawn) true)
    (CallFunction|SetIgnoreInput true)
    (Transformation|SetActorLocationAndRotation (Variables|Default|GetFrogPawn) (Transformation|GetActorLocation Home) (Transformation|GetActorRotation Home) false true)
    (CallFunction|AddPoints (+ (* (Math|Float|Floor (- (Variables|Default|GetTimerMaxSeconds) (Variables|/Script/RoadToad.RoadToadGameState|GetDEPR_GameTimerSecondsLeft (Variables|Default|GetRoadToadGameState)))) 10) 50))
    (Default|CloseHome Home)
    (if (>= (Utilities|Array|Length (Class|RoadToadGameState|GetOccupiedHomes (Variables|Default|GetRoadToadGameState))) 5)
      (Class|RoadToadHUD|ShowLevelComplete (Variables|Default|GetRoadToadHUD) (Class|RoadToadGameState|GetCurrentLevel (Variables|Default|GetRoadToadGameState)))
      (Variables|Default|SetCanStartNextLevel true)
      (else
        (Utilities|FlowControl|Delay 1.0)
        (CallFunction|RespawnFrog)))))

(event Custom|RespawnFrog
  ;[0 1 0] frog life cycle
  (CallFunction|TickJumpTimer (Variables|Default|GetJumpTimerMaxSeconds))
  (bind _returnvalue (Game|SpawnActorfromClass "/Game/RoadToad/Blueprints/BP_ThirdPersonFrog.BP_ThirdPersonFrog_C" (Transformation|GetActorTransform (Class|GameModeBase|FindPlayerStart (Game|GetPlayerController 0))) "AlwaysSpawn" "MultiplyWithRoot" 0 0))
  (Actor|DestroyActor (Variables|Default|GetFrogPawn))
  (bind _output_get (Variables|Default|SetFrogPawn _returnvalue))
  (Pawn|Possess (Game|GetPlayerController 0) _output_get)
  (Rendering|SetActorHiddenInGame (Variables|Default|GetFrogPawn) false)
  (Class|RoadToadHUD|HideDeathUI (Variables|Default|GetRoadToadHUD))
  (Variables|/Script/Engine.PostProcessVolume|SetSettings (Variables|Default|GetPostProcessVolume) (Utilities|Struct|MakePostProcessSettings (Math|Vector4|MakeVector4 1.0 1.0 1.0 1.0)))
  (Utilities|Time|SetGlobalTimeDilation 1.0)
  (Physics|SetSimulatePhysics (Variables|/Script/Engine.Character|GetCapsuleComponent (Variables|Default|GetFrogPawn)) false)
  (CallFunction|SetIgnoreInput false)
  (CallFunction|RestartTimer)
  (CallFunction|AllowDeath)
  (Class|RoadToadHUD|ShowBottomPanel (Variables|Default|GetRoadToadHUD))
  (Default|RemoveBubble (Variables|Default|GetFrogPawn))
  (CallFunction|ResetMovablesSpeed true)
  (for _array_element (Variables|Default|GetCars)
    (Default|Enable _array_element)
    (bind _asbp_powerup_slow (Utilities|Casting|CastToBP_Powerup_Slow (Variables|/Script/Engine.ChildActorComponent|GetChildActor (Variables|/Game/RoadToad/Blueprints/Movables/BP_Car.BP_Car_C|GetPowerup_Slow _array_element))))
    (Default|Disable _asbp_powerup_slow)
    (bind _asbp_powerup_bubble (Utilities|Casting|CastToBP_Powerup_Bubble (Variables|/Script/Engine.ChildActorComponent|GetChildActor (Variables|/Game/RoadToad/Blueprints/Movables/BP_Car.BP_Car_C|GetPowerup_Bubble _array_element))))
    (Default|Disable _asbp_powerup_bubble))
  (for _array_element_2 (Variables|Default|GetLogs)
    (bind _asbp_power_up (Utilities|Casting|CastToBP_PowerUp (Variables|/Script/Engine.ChildActorComponent|GetChildActor (Variables|/Game/RoadToad/Blueprints/Movables/BP_Log.BP_Log_C|GetPowerup _array_element_2))))
    (Default|Disable _asbp_power_up))
  (for _array_element_3 (Variables|Default|GetTurtleChains)
    (bind _asbp_power_up_2 (Utilities|Casting|CastToBP_PowerUp (Variables|/Script/Engine.ChildActorComponent|GetChildActor (Variables|/Game/RoadToad/Blueprints/Movables/BP_TurtleChain.BP_TurtleChain_C|GetPowerup _array_element_3))))
    (Default|Disable _asbp_power_up_2)))

(event Custom|SpawnPowerup
  ;[1 0 1] powerup
  (if (Math|Random|RandomBoolwithWeight (Variables|Default|GetPowerupRandomWeight))
    (Variables|Default|SetPowerupRandomWeight (- (Variables|Default|GetPowerupRandomWeight) 1.0))
    (else
      (Variables|Default|SetPowerupRandomWeight (+ (Variables|Default|GetPowerupRandomWeight) 1.0))))
  (Default|Enable (CallFunction|ChoosePowerupSpawnPoint)))

(event Custom|TriggerSpawnPowerup
  ;[1 0 1] powerup
  (Utilities|FlowControl|Delay (Math|Random|RandomFloatinRange 2.0 6.0))
  (CallFunction|SpawnPowerup))

(event Custom|ToggleNightMode
  ;[1 0 1] Powerup (night mode)
  (bind _isa (Utilities|FlowControl|FlipFlop)
    (:A
      _)
    (:B
      _))
  (Variables|Default|SetNightMode _isa)
  (if (Variables|Default|GetNightMode)
    (bind _alpha (Timeline|FadeToNight PlayFromStart)
      (:Update
        (Rendering|Components|Light|SetLightColor (Variables|/Script/Engine.Light|GetLightComponent (Variables|Default|GetSunLight)) (Math|Color|Lerp(LinearColor) "(R=1.000000,G=1.000000,B=1.000000,A=1.000000)" (Variables|Default|GetNightLightColor) _alpha) true)
        (Rendering|Components|Light|SetIntensity (Variables|/Script/Engine.Light|GetLightComponent (Variables|Default|GetFrontalLight)) (- 1.0 _alpha)))
      (:Headlights
        (for _array_element (Variables|Default|GetCars)
          (if (Variables|/Game/RoadToad/Blueprints/Movables/BP_Movable.BP_Movable_C|GetEnabled _array_element)
            (Rendering|SetVisibility (Variables|/Game/RoadToad/Blueprints/Movables/BP_Car.BP_Car_C|GetSpotLight _array_element) (Variables|Default|GetNightMode) false)))))
    (else
      (Timeline|FadeToNight ReverseFromEnd))))

(event Custom|SlowMovables
  (bind _nightmode (Variables|Default|GetNightMode))
  ;[1 0 1] Powerup (slowmo)
  (Variables|Default|SetWasNightModeBeforeSlow _nightmode)
  (if _nightmode
    _
    (else
      (CallFunction|SwitchtoNight)))
  (for _array_element (Variables|Default|GetMovables)
    (if (Variables|/Game/RoadToad/Blueprints/Movables/BP_Movable.BP_Movable_C|GetEnabled _array_element)
      (if (not (Variables|/Game/RoadToad/Blueprints/Movables/BP_Movable.BP_Movable_C|GetSlowed _array_element))
        (Variables|/Game/RoadToad/Blueprints/Movables/BP_Movable.BP_Movable_C|SetSpeed _array_element (/ (Variables|/Game/RoadToad/Blueprints/Movables/BP_Movable.BP_Movable_C|GetSpeed _array_element) (Variables|Default|GetMovableSlowingFactor)))
        (Variables|/Game/RoadToad/Blueprints/Movables/BP_Movable.BP_Movable_C|SetSlowed _array_element true))))
  (Audio|Components|Audio|SetPitchMultiplier (Variables|/Script/Engine.AmbientSound|GetAudioComponent (Variables|Default|GetMusicActor)) 0.5)
  (Utilities|FlowControl|Delay 5.0)
  (CallFunction|ResetMovablesSpeed false)
  (CallFunction|TriggerSpawnPowerup))

(event Custom|ResetMovablesSpeed
  (params (CalledByRespawn :type Boolean))
  ;[1 0 1] Powerup (slowmo)
  (if CalledByRespawn
    _
    (elif (Variables|Default|GetWasNightModeBeforeSlow)
      _
      (else
        (CallFunction|SwitchtoDay))))
  (for _array_element (Variables|Default|GetMovables)
    (if (Variables|/Game/RoadToad/Blueprints/Movables/BP_Movable.BP_Movable_C|GetEnabled _array_element)
      (if (Variables|/Game/RoadToad/Blueprints/Movables/BP_Movable.BP_Movable_C|GetSlowed _array_element)
        (Variables|/Game/RoadToad/Blueprints/Movables/BP_Movable.BP_Movable_C|SetSpeed _array_element (* (Variables|/Game/RoadToad/Blueprints/Movables/BP_Movable.BP_Movable_C|GetSpeed _array_element) (Variables|Default|GetMovableSlowingFactor)))
        (Variables|/Game/RoadToad/Blueprints/Movables/BP_Movable.BP_Movable_C|SetSlowed _array_element false))))
  (Audio|Components|Audio|SetPitchMultiplier (Variables|/Script/Engine.AmbientSound|GetAudioComponent (Variables|Default|GetMusicActor)) 1.0))

(event Custom|TryStartNextLevel
  ;[1 0 0] game flow
  (if (Variables|Default|GetCanStartNextLevel)
    (Variables|Default|SetCanStartNextLevel false)
    (Class|RoadToadHUD|HideLevelComplete (Variables|Default|GetRoadToadHUD))
    (bind _returnvalue (Class|RoadToadGameState|IncrementLevel (Variables|Default|GetRoadToadGameState)))
    (Class|RoadToadHUD|UpdateLevelNumber (Variables|Default|GetRoadToadHUD) _returnvalue)
    (Variables|Default|SetNewPointsMultiplier (* (Variables|Default|GetNewPointsMultiplier) 1.25))
    (for _array_element (Variables|Default|GetMovables)
      (Variables|/Game/RoadToad/Blueprints/Movables/BP_Movable.BP_Movable_C|SetSpeed _array_element (* (Variables|/Game/RoadToad/Blueprints/Movables/BP_Movable.BP_Movable_C|GetSpeed _array_element) 1.25)))
    (Variables|Default|SetCanRestart true)
    (CallFunction|TryRestart false)))

(event Custom|FrogMadeFirstMove
  ;[1 0 0] game flow
  (CallFunction|TriggerSpawnPowerup)
  (CallFunction|RestartTimer))

(event Custom|RestartJumpTimer
  (bind _returnvalue (Math|Float|MakeLiteralFloat 0.1))
  ;[1 1 0] timers
  (Variables|Default|SetJumpTimerEnabled true)
  (Variables|/Script/RoadToad.RoadToadGameState|SetDEPR_JumpTimerSeconds (Variables|Default|GetRoadToadGameState) 0.0)
  (Class|RoadToadHUD|UpdateJumpTimer (Variables|Default|GetRoadToadHUD) 0.0)
  (Utilities|FlowControl|Delay _returnvalue :!label _label)
  (if (Variables|Default|GetJumpTimerEnabled)
    (CallFunction|TickJumpTimer _returnvalue)
    (goto _label)))

(event Custom|TickJumpTimer
  (params (SecondsPassed :type Float%20%28double-precision%29))
  (bind _roadtoadgamestate (Variables|Default|GetRoadToadGameState))
  ;[1 1 0] timers
  (bind _output_get (Variables|/Script/RoadToad.RoadToadGameState|SetDEPR_JumpTimerSeconds _roadtoadgamestate (+ (Variables|/Script/RoadToad.RoadToadGameState|GetDEPR_JumpTimerSeconds _roadtoadgamestate) SecondsPassed)))
  (Class|RoadToadHUD|UpdateJumpTimer (Variables|Default|GetRoadToadHUD) (/ _output_get (Variables|Default|GetJumpTimerMaxSeconds)))
  (if (>= (/ _output_get (Variables|Default|GetJumpTimerMaxSeconds)) 1.0)
    (Variables|Default|SetCanJump true)))

(event Custom|SwitchToDay
  ;[1 0 1] Powerup (night mode)
  (Variables|Default|SetNightMode false)
  (if (Variables|Default|GetNightMode)
    (bind _alpha (Timeline|FadeToNight PlayFromStart)
      (:Update
        (Rendering|Components|Light|SetLightColor (Variables|/Script/Engine.Light|GetLightComponent (Variables|Default|GetSunLight)) (Math|Color|Lerp(LinearColor) "(R=1.000000,G=1.000000,B=1.000000,A=1.000000)" (Variables|Default|GetNightLightColor) _alpha) true)
        (Rendering|Components|Light|SetIntensity (Variables|/Script/Engine.Light|GetLightComponent (Variables|Default|GetFrontalLight)) (- 1.0 _alpha)))
      (:Headlights
        (for _array_element (Variables|Default|GetCars)
          (if (Variables|/Game/RoadToad/Blueprints/Movables/BP_Movable.BP_Movable_C|GetEnabled _array_element)
            (Rendering|SetVisibility (Variables|/Game/RoadToad/Blueprints/Movables/BP_Car.BP_Car_C|GetSpotLight _array_element) (Variables|Default|GetNightMode) false)))))
    (else
      (Timeline|FadeToNight ReverseFromEnd))))

(event Custom|FrogDied
  (params (Cause%20Of%20Death :type ECauseOfDeath%20Enum :default "Car"))
  (bind _frogpawn (Variables|Default|GetFrogPawn))
  ;[0 1 0] toad life cycle
  (Utilities|FlowControl|Gate false
    (:Exit
      (CallFunction|SwitchtoOutcomeCamera)
      (Class|AudioSubsystem|PlaySound (Subsystems|GetAudioSubsystem) (Utilities|Select :Index Cause%20Of%20Death :Car "/Game/RoadToad/Sounds/SW_Splat.SW_Splat" :Water "/Game/RoadToad/Sounds/SW_Splash.SW_Splash" :Timer "/Game/RoadToad/Sounds/SW_Ribbit.SW_Ribbit") (Utilities|Select :Index Cause%20Of%20Death :Car 1.0 :Water 1.0 :Timer 0.5))
      (CallFunction|ProhibitDeath)
      (if (Utilities|Enum|Equal(Enum) Cause%20Of%20Death "Car")
        (Default|Flatten (Variables|Default|GetFrogPawn)))
      (CallFunction|StopTimer)
      (Class|RoadToadHUD|HideBottomPanel (Variables|Default|GetRoadToadHUD))
      (CallFunction|SetIgnoreInput true)
      (Variables|/Script/Engine.PostProcessVolume|SetSettings (Variables|Default|GetPostProcessVolume) (Utilities|Struct|MakePostProcessSettings (Math|Vector4|MakeVector4 0.5 0.5 0.5 0.5)))
      (Default|StopJumpAnimation _frogpawn)
      (Physics|SetSimulatePhysics (Variables|/Script/Engine.Character|GetCapsuleComponent _frogpawn) true)
      (bind _returnvalue (Class|RoadToadGameState|TakeALife (Variables|Default|GetRoadToadGameState)))
      (Class|RoadToadHUD|UpdateLivesLeft (Variables|Default|GetRoadToadHUD) _returnvalue)
      (Utilities|Time|SetGlobalTimeDilation 0.1)
      (if (>= _returnvalue 0)
        (Class|RoadToadHUD|ShowDeathUI (Variables|Default|GetRoadToadHUD) Cause%20Of%20Death)
        (Utilities|FlowControl|Delay 0.15)
        (CallFunction|RespawnFrog)
        (else
          (EventDispatchers|BindEventtoRetryReady (Variables|Default|GetRoadToadHUD) (delegate Custom|RetryReady)))))))

(event Custom|SwitchToNight
  ;[1 0 1] Powerup (night mode)
  (Variables|Default|SetNightMode true)
  (if (Variables|Default|GetNightMode)
    (bind _alpha (Timeline|FadeToNight PlayFromStart)
      (:Update
        (Rendering|Components|Light|SetLightColor (Variables|/Script/Engine.Light|GetLightComponent (Variables|Default|GetSunLight)) (Math|Color|Lerp(LinearColor) "(R=1.000000,G=1.000000,B=1.000000,A=1.000000)" (Variables|Default|GetNightLightColor) _alpha) true)
        (Rendering|Components|Light|SetIntensity (Variables|/Script/Engine.Light|GetLightComponent (Variables|Default|GetFrontalLight)) (- 1.0 _alpha)))
      (:Headlights
        (for _array_element (Variables|Default|GetCars)
          (if (Variables|/Game/RoadToad/Blueprints/Movables/BP_Movable.BP_Movable_C|GetEnabled _array_element)
            (Rendering|SetVisibility (Variables|/Game/RoadToad/Blueprints/Movables/BP_Car.BP_Car_C|GetSpotLight _array_element) (Variables|Default|GetNightMode) false)))))
    (else
      (Timeline|FadeToNight ReverseFromEnd))))

(event Custom|ShowHUD
  (Class|RootWidget|ShowHUD (Variables|Default|GetRootWidget)))

(event Custom|Pause
  (Game|SetGamePaused true)
  (Class|RootWidget|ShowPauseMenu (Variables|Default|GetRootWidget)))

(event Custom|RetryReady
  ;[0 1 0] toad life cycle
  (EventDispatchers|UnbindEventfromRetryReady (Variables|Default|GetRoadToadHUD) (delegate Custom|RetryReady))
  (Variables|Default|SetCanRestart true))

(event Custom|SwitchToOutcomeCamera
  (Utilities|IsValid (Variables|Default|GetOutcomeCam)
    (:Is%20Valid
      _)
    (:Is%20Not%20Valid
      (bind _outactors (Actor|GetAllActorsOfClasswithTag "/Script/Engine.CameraActor" "Outcome"))
      (Variables|Default|SetOutcomeCam (Utilities|Array|Get(acopy) _outactors))))
  (bind _desiredview (Class|CameraComponent|GetCameraView (Variables|/Game/RoadToad/Blueprints/BP_ThirdPersonFrog.BP_ThirdPersonFrog_C|GetFollowCamera (Variables|Default|GetFrogPawn)) 0.0))
  (Transformation|SetActorLocationAndRotation (Variables|Default|GetOutcomeCam) (.Location (Utilities|Struct|BreakMinimalViewInfo _desiredview)) (Math|Rotator|FindLookatRotation (.Location (Utilities|Struct|BreakMinimalViewInfo _desiredview)) (Transformation|GetActorLocation (Pawn|GetControlledPawn (Game|GetPlayerController 0)))))
  (Game|Player|SetViewTargetwithBlend (Game|GetPlayerController 0) (Variables|Default|GetOutcomeCam) 0.0 "VTBlend_Linear" 0.0 false))

(event Custom|SetIgnoreInput
  (params (NewIgnore :type Boolean))
  (bind _returnvalue (Game|GetPlayerController 0))
  (Input|SetIgnoreMoveInput _returnvalue NewIgnore)
  (Input|SetIgnoreLookInput _returnvalue NewIgnore))

(event Custom|NextLevel
  ;[1 0 0] game flow
  (Class|RoadToadHUD|ShowLevelComplete (Variables|Default|GetRoadToadHUD) (Class|RoadToadGameState|GetCurrentLevel (Variables|Default|GetRoadToadGameState)))
  (Variables|Default|SetCanStartNextLevel true))

(event Custom|OpenExitGameMenu
  (Default|ShowExitGameMenu (Variables|Default|GetRootWidget)))

(event Custom|HighScoreLoaded
  (params (HighScore :type Integer))
  (bind _output_get (Variables|/Script/RoadToad.RoadToadGameState|SetHighScore (Variables|Default|GetRoadToadGameState) HighScore))
  (Class|RoadToadHUD|UpdateHighScore (Variables|Default|GetRoadToadHUD) _output_get))

(event Custom|RestartTimer
  (bind _returnvalue (Math|Float|MakeLiteralFloat 0.1))
  ;[1 1 0] timers
  (Variables|Default|SetTimerEnabled true)
  (Variables|/Script/RoadToad.RoadToadGameState|SetDEPR_GameTimerSecondsLeft (Variables|Default|GetRoadToadGameState) (Variables|Default|GetTimerMaxSeconds))
  (Class|RoadToadHUD|UpdateLifeTimer (Variables|Default|GetRoadToadHUD) 1.0)
  (Utilities|FlowControl|Delay _returnvalue :!label _label)
  (if (Variables|Default|GetTimerEnabled)
    (CallFunction|TickTimer _returnvalue)
    (goto _label)))

(event Custom|TickTimer
  (params (SecondsPassed :type Float%20%28double-precision%29))
  (bind _roadtoadgamestate (Variables|Default|GetRoadToadGameState))
  ;[1 1 0] timers
  (bind _output_get (Variables|/Script/RoadToad.RoadToadGameState|SetDEPR_GameTimerSecondsLeft _roadtoadgamestate (- (Variables|/Script/RoadToad.RoadToadGameState|GetDEPR_GameTimerSecondsLeft _roadtoadgamestate) SecondsPassed)))
  (Class|RoadToadHUD|UpdateLifeTimer (Variables|Default|GetRoadToadHUD) (/ _output_get (Variables|Default|GetTimerMaxSeconds)))
  (if (<= (/ _output_get (Variables|Default|GetTimerMaxSeconds)) 0.0)
    (CallFunction|FrogDied "Timer")))

(event Custom|ProhibitDeath
  (bind _frogpawn (Variables|Default|GetFrogPawn))
  ;[0 1 0] toad life cycle
  (Utilities|FlowControl|Gate false) ; enters at Close
)

(event Custom|AllowDeath
  (bind _frogpawn (Variables|Default|GetFrogPawn))
  ;[0 1 0] toad life cycle
  (Utilities|FlowControl|Gate false) ; enters at Open
)

(event Custom|AddPoints
  (params (Points :type Integer))
  (bind _roadtoadhud (Variables|Default|GetRoadToadHUD))
  ;[0 1 1] scoring
  (bind _returnvalue (Class|RoadToadGameState|AddPoints (Variables|Default|GetRoadToadGameState) (Math|Float|Round (* Points (Variables|Default|GetNewPointsMultiplier)))))
  (Class|RoadToadHUD|UpdateScore _roadtoadhud _returnvalue)
  (Class|RoadToadHUD|UpdateHighScore _roadtoadhud (Variables|/Script/RoadToad.RoadToadGameState|GetHighScore (Variables|Default|GetRoadToadGameState))))

(event Custom|StopTimer
  ;[1 1 0] timers
  (Variables|Default|SetTimerEnabled false))

(event Custom|TryRestart
  (params (ResetScore :type Boolean))
  (bind _roadtoadgamestate (Variables|Default|GetRoadToadGameState))
  ;[1 0 0] game flow
  (if (Variables|Default|GetCanRestart)
    (Variables|Default|SetCanRestart false)
    (if ResetScore
      (Class|RoadToadGameState|ClearScore (Variables|Default|GetRoadToadGameState))
      (Class|RoadToadHUD|UpdateScore (Variables|/Game/RoadToad/Blueprints/Widgets/WBP_Root.WBP_Root_C|GetHUD (Variables|Default|GetRootWidget))))
    (Class|RoadToadGameState|EmptyOccupiedHomes _roadtoadgamestate)
    (Class|RoadToadGameState|ResetLives _roadtoadgamestate)
    (Class|RoadToadHUD|ResetUI (Variables|Default|GetRoadToadHUD))
    (for _array_element (Variables|Default|GetFrogHomes)
      (Default|OpenHome _array_element))
    (for _array_element_2 (Variables|Default|GetCars)
      (if (not (Variables|/Game/RoadToad/Blueprints/Movables/BP_Movable.BP_Movable_C|GetEnabled _array_element_2))
        (Default|Enable _array_element_2)))
    (CallFunction|RespawnFrog)))

(event EventBeginPlay
  (bind _returnvalue (UserInterface|CreateWidget "/Game/RoadToad/Blueprints/Widgets/WBP_Root.WBP_Root_C"))
  (bind _output_get (Variables|Default|SetRootWidget _returnvalue))
  (UserInterface|Viewport|AddtoViewport _output_get 0)
  (Class|RootWidget|ShowPauseMenu (Variables|Default|GetRootWidget))
  (Class|RootWidget|HideHUD (Variables|Default|GetRootWidget))
  (Class|Actor|SetTickablewhenPaused true)
  (Variables|Default|SetRoadToadHUD (Class|RootWidget|GetHUD (Variables|Default|GetRootWidget)))
  (bind _outactors (Actor|GetAllActorsOfClasswithTag "/Script/Engine.CameraActor" "Startup"))
  (Game|Player|SetViewTargetwithBlend (Game|GetPlayerController 0) (Utilities|Array|Get(acopy) _outactors) 0.0 "VTBlend_Linear" 0.0 false)
  (bind _outactors_2 (Actor|GetAllActorsOfClasswithTag "/Script/Engine.DirectionalLight" "sun"))
  (Variables|Default|SetSunLight (Utilities|Array|Get(acopy) _outactors_2))
  (CallFunction|SetIgnoreInput true)
  (Variables|/Script/Engine.PlayerController|SetbShowMouseCursor (Game|GetPlayerController 0) true)
  (bind _outactors_3 (Actor|GetAllActorsOfClasswithTag "/Script/Engine.DirectionalLight" "front"))
  (Variables|Default|SetFrontalLight (Utilities|Array|Get(acopy) _outactors_3))
  (bind _returnvalue_2 (Actor|GetActorOfClass "/Script/Engine.PostProcessVolume"))
  (Variables|Default|SetPostProcessVolume _returnvalue_2)
  (bind _asroad_toad_game_state (Utilities|Casting|CastToRoadToadGameState (Game|GetGameState)))
  (Variables|Default|SetRoadToadGameState _asroad_toad_game_state)
  (bind _asbp_third_person_frog (Utilities|Casting|CastToBP_ThirdPersonFrog (Game|Player|GetPlayerPawn 0)))
  (Variables|Default|SetFrogPawn _asbp_third_person_frog)
  (bind _outactors_4 (Actor|GetAllActorsOfClass "/Game/RoadToad/Blueprints/Movables/BP_Home.BP_Home_C"))
  (Variables|Default|SetFrogHomes _outactors_4)
  (bind _outactors_5 (Actor|GetAllActorsOfClass "/Game/RoadToad/Blueprints/Movables/BP_Movable.BP_Movable_C"))
  (bind _output_get_2 (Variables|Default|SetMovables _outactors_5))
  (for _array_element _output_get_2
    (bind _asbp_car (Utilities|Casting|CastToBP_Car _array_element)
      (:then
        (Utilities|Array|Add (Variables|Default|GetCars) _asbp_car))
      (:CastFailed
        (bind _asbp_log (Utilities|Casting|CastToBP_Log _array_element)
          (:then
            (Utilities|Array|Add (Variables|Default|GetLogs) _asbp_log))
          (:CastFailed
            (bind _asbp_turtle_chain (Utilities|Casting|CastToBP_TurtleChain _array_element))
            (Utilities|Array|Add (Variables|Default|GetTurtleChains) _asbp_turtle_chain))))))
  (bind _returnvalue_3 (Actor|GetActorOfClass "/Script/Engine.AmbientSound"))
  (Variables|Default|SetMusicActor _returnvalue_3))

(fn ConstructionScript)

(fn FindPlayerStart
  (params (Player :type Controller%20Object%20Reference) (IncomingName :type String))
  (if (== (Utilities|Array|Length (Variables|Default|GetPlayerStarts)) 0)
    (bind _outactors (Actor|GetAllActorsOfClass "/Script/Engine.PlayerStart"))
    (Variables|Default|SetPlayerStarts _outactors))
  (return (Utilities|Array|Get(acopy) (Variables|Default|GetPlayerStarts) (Math|Random|RandomIntegerinRange 0 (Utilities|Array|LastIndex (Variables|Default|GetPlayerStarts))))))

(fn ChoosePowerupSpawnPoint
  (bind _logs (Variables|Default|GetLogs))
  (bind _turtlechains (Variables|Default|GetTurtleChains))
  (bind _cars (Variables|Default|GetCars))
  (bind _returnvalue (Utilities|Array|LastIndex _cars))
  (bind _returnvalue_2 (Math|Random|RandomIntegerinRange 0 _returnvalue))
  (bind _output (Utilities|Array|Get(acopy) _cars _returnvalue_2))
  (if (>= (Variables|/Game/RoadToad/Blueprints/BP_ThirdPersonFrog.BP_ThirdPersonFrog_C|GetThisFrogDistanceRecord (Variables|Default|GetFrogPawn)) 5e+02)
    (bind _asbp_power_up (Utilities|Casting|CastToBP_PowerUp (Utilities|SelectObject (Variables|/Script/Engine.ChildActorComponent|GetChildActor (Variables|/Game/RoadToad/Blueprints/Movables/BP_TurtleChain.BP_TurtleChain_C|GetPowerup (Utilities|Array|Get(acopy) _turtlechains (Math|Random|RandomIntegerinRange 0 (Utilities|Array|LastIndex _turtlechains))))) (Variables|/Script/Engine.ChildActorComponent|GetChildActor (Variables|/Game/RoadToad/Blueprints/Movables/BP_Log.BP_Log_C|GetPowerup (Utilities|Array|Get(acopy) _logs (Math|Random|RandomIntegerinRange 0 (Utilities|Array|LastIndex _logs))))) (Math|Random|RandomBool))))
    (return _asbp_power_up)
    (else
      (bind _asbp_power_up_2 (Utilities|Casting|CastToBP_PowerUp (select (Math|Random|RandomBoolwithWeight (Variables|Default|GetPowerupRandomWeight)) (Variables|/Script/Engine.ChildActorComponent|GetChildActor (Variables|/Game/RoadToad/Blueprints/Movables/BP_Car.BP_Car_C|GetPowerup_Slow _output)) (Variables|/Script/Engine.ChildActorComponent|GetChildActor (Variables|/Game/RoadToad/Blueprints/Movables/BP_Car.BP_Car_C|GetPowerup_Bubble _output)))))
      (return _asbp_power_up_2))))