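; BP_TurtleChain is a Frogger actor representing a chain of three turtle shells that can optionally dive.
; On BeginPlay it waits a random delay of up to one second, staggering instances, then plays a timeline if WillDive is set.
; The timeline's Height track offsets the whole actor vertically from its starting Z, while its Tilt track pitches all three shell meshes together.
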(event EventBeginPlay
  (bind _returnvalue (Transformation|GetActorLocation))
  (|CallParentFunction)
  (Utilities|FlowControl|Delay (Math|Random|RandomFloatinRange 0.0 1.0))
  (if (Variables|Default|GetWillDive)
    (Variables|Default|SetInitialHeight (.z (Transformation|GetActorLocation)))
    (bind (_direction _height _tilt) (Timeline|Timeline_0 Play)
      (:Update
        (Transformation|SetActorLocation (Math|Vector|MakeVector (.x _returnvalue) (.y _returnvalue) (+ (* _height 125.0) (Variables|Default|GetInitialHeight))) false false)
        (Transformation|SetRelativeRotation (Variables|Default|GetSM_TurtleShell) (Math|Rotator|MakeRotator 0.0 _tilt 0.0) false false)))))

(fn ConstructionScript
  (|CallParentFunction))