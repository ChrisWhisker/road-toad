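; BP_PowerUp is a Frogger power-up actor, shown as a star that can be switched on and off.
; Enable shows the star, turns on the box collision and plays a timeline that scales the star relative to its original size.
; Disable hides the star and turns off collision, while Tick spins the star only while enabled.
; BeginPlay caches the star's scale and applies the initial Enabled state.
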(event Custom|Enable
  (Rendering|SetVisibility (Variables|Default|Getstar) true false)
  (Collision|SetCollisionEnabled (Variables|Default|GetBox) "QueryAndPhysics")
  (Variables|Default|SetEnabled true)
  (bind _newtrack_0 (Timeline|Timeline_0 Play)
    (:Update
      (Transformation|SetRelativeScale3D (Variables|Default|Getstar) (* (Variables|Default|GetOriginalScale) _newtrack_0)))))

(event Custom|Disable
  (Rendering|SetVisibility (Variables|Default|Getstar) false false)
  (Collision|SetCollisionEnabled (Variables|Default|GetBox) "NoCollision")
  (Variables|Default|SetEnabled false))

(event EventBeginPlay
  (Variables|Default|SetOriginalScale (Variables|/Script/Engine.SceneComponent|GetRelativeScale3D (Variables|Default|Getstar)))
  (if (Variables|Default|GetEnabled)
    (CallFunction|Enable)
    (else
      (Collision|SetCollisionEnabled (Variables|Default|GetBox) "NoCollision"))))

(event EventTick
  (params (DeltaSeconds :type Float%20%28single-precision%29))
  (if (Variables|Default|GetEnabled)
    (Transformation|AddLocalRotation (Variables|Default|Getstar) (Math|Rotator|MakeRotator 0.0 0.0 (* DeltaSeconds (Variables|Default|GetSpinSpeed))) false false)))

(fn ConstructionScript)