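; BP_Movable is a Frogger actor that moves along the X axis and wraps around at the edges of the play area.
; While enabled, Tick offsets X by Speed scaled by delta time, using GameHalfWidth from the cached FroggerGameMode as the boundary.
; Crossing either edge teleports it to the opposite side and calls Respawn, an empty event that serves as a hook.
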(event Custom|Respawn)

(event EventTick
  (params (DeltaSeconds :type Float%20%28single-precision%29))
  (bind _returnvalue (Transformation|GetActorLocation))
  (bind _froggergamemode (Variables|Default|GetFroggerGameMode))
  (bind _gamehalfwidth (Variables|/Game/Frogger/Blueprints/FroggerGameMode.FroggerGameMode_C|GetGameHalfWidth _froggergamemode))
  (bind _returnvalue_2 (* _gamehalfwidth -1.0))
  (if (Variables|Default|GetEnabled)
    (if (> (.x _returnvalue) (Variables|/Game/Frogger/Blueprints/FroggerGameMode.FroggerGameMode_C|GetGameHalfWidth (Variables|Default|GetFroggerGameMode)))
      (Transformation|SetActorLocation (Math|Vector|MakeVector _returnvalue_2 (.y _returnvalue) (.z _returnvalue)) false true)
      (CallFunction|Respawn)
      (elif (< (.x _returnvalue) _returnvalue_2)
        (Transformation|SetActorLocation (Math|Vector|MakeVector (Variables|/Game/Frogger/Blueprints/FroggerGameMode.FroggerGameMode_C|GetGameHalfWidth (Variables|Default|GetFroggerGameMode)) (.y _returnvalue) (.z _returnvalue)) false true)
        (CallFunction|Respawn)
        (else
          (Transformation|SetActorLocation (Math|Vector|MakeVector (+ (* DeltaSeconds (Variables|Default|GetSpeed)) (.x _returnvalue)) (.y _returnvalue) (.z _returnvalue)) false false))))))

(event EventBeginPlay
  (|CallParentFunction)
  (bind _asfrogger_game_mode (Utilities|Casting|CastToFroggerGameMode (Game|GetGameMode)))
  (Variables|Default|SetFroggerGameMode _asfrogger_game_mode))

(fn ConstructionScript)