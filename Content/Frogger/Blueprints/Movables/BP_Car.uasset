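; BP_Car is a Frogger movable car with randomized paint hue, headlight tint and horn voice, honking at the player frog.
; One shared dynamic material colors the body and is re-hued on Respawn.
; Enable and Disable toggle collision and visibility for pooling-style reuse.
; The honk trigger has a one-second cooldown, lowers pitch when slowed, plays a roof-scale timeline and boosts headlights in night mode.
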(event OnComponentBeginOverlap(HonkTrigger)
  (params (OverlappedComponent :type Primitive%20Component%20Object%20Reference) (OtherActor :type Actor%20Object%20Reference) (OtherComp :type Primitive%20Component%20Object%20Reference) (OtherBodyIndex :type Integer) (bFromSweep :type Boolean) (SweepResult :type Hit%20Result%20Structure%20%28by%20ref%29))
  (bind _returnvalue (Math|Float|MakeLiteralFloat 5e+03))
  (bind _returnvalue_2 (Math|Float|MakeLiteralFloat 1.5e+04))
  (Utilities|Casting|CastToBP_ThirdPersonFrog OtherActor)
  (Utilities|FlowControl|DoOnce false :!label _label
    (:Completed
      (Class|AudioSubsystem|PlaySound (Subsystems|GetAudioSubsystem) (select (Variables|Default|GetUseDoubleHonk) "/Game/Frogger/Sounds/SW_HonkHonk.SW_HonkHonk" "/Game/Frogger/Sounds/SW_Honk.SW_Honk") (* (select (Variables|Default|GetSlowed) 0.5 1.0) (Variables|Default|GetHornPitch)))
      (Utilities|FlowControl|Sequence
        (:then_0
          (Utilities|FlowControl|Delay 1.0)
          (goto _label Reset))
        (:then_1
          (if (Variables|/Game/Frogger/Blueprints/FroggerGameMode.FroggerGameMode_C|GetNightMode (Variables|Default|GetFroggerGameMode))
            (Rendering|Components|Light|SetIntensity (Variables|Default|GetSpotLight) _returnvalue_2)
            (Rendering|Components|Light|SetIntensity (Variables|Default|GetSpotLight1) _returnvalue_2)
            (bind _scale (Timeline|HonkEffect PlayFromStart)
              (:Update
                (Transformation|SetRelativeScale3D (Variables|Default|GetRoof) (* _scale (Variables|Default|GetOrigRoofScale))))
              (:Finished
                (Rendering|Components|Light|SetIntensity (Variables|Default|GetSpotLight) _returnvalue)
                (Rendering|Components|Light|SetIntensity (Variables|Default|GetSpotLight1) _returnvalue)))
            (else
              (Timeline|HonkEffect PlayFromStart))))))))

(event Custom|Disable
  (bind _tirefr (Variables|Default|GetTireFR))
  (Collision|SetCollisionEnabled _tirefr "NoCollision")
  (Rendering|SetVisibility _tirefr false false)
  (Variables|Default|SetEnabled false)
  (Rendering|SetVisibility (Variables|Default|GetSpotLight) false false))

(event Custom|Enable
  (bind _tirefr (Variables|Default|GetTireFR))
  (Collision|SetCollisionEnabled _tirefr "QueryAndPhysics")
  (Rendering|SetVisibility _tirefr true false)
  (Variables|Default|SetEnabled true))

(event EventBeginPlay
  (|CallParentFunction)
  (bind _returnvalue (Rendering|Material|CreateDynamicMaterialInstance (Utilities|Array|Get(acopy) (Rendering|Material|GetMaterials (Variables|Default|GetChassis))) "None" "None" :!class /Script/Engine.KismetMaterialLibrary))
  (bind _output_get (Variables|Default|SetDMI _returnvalue))
  (Rendering|Material|SetMaterial (Variables|Default|GetChassis) 0 _output_get)
  (CallFunction|Respawn)
  (Rendering|Components|Light|SetLightColor (Variables|Default|GetSpotLight) (select (Math|Random|RandomBool) "(R=1.000000,G=1.000000,B=0.333000,A=1.000000)" "(R=1.000000,G=1.000000,B=1.000000,A=1.000000)") true)
  (Variables|Default|SetHornPitch (Math|Random|RandomFloatinRange 0.75 1.25))
  (Variables|Default|SetUseDoubleHonk (Math|Random|RandomBool))
  (Variables|Default|SetOrigRoofScale (Variables|/Script/Engine.SceneComponent|GetRelativeScale3D (Variables|Default|GetRoof))))

(event EventRespawn
  (Variables|Default|SetPaintColor (Math|Color|MakeColor 1.0 1.0 1.0))
  (Class|KismetMathLibrary|LinearColorSetRandomHue (Variables|Default|GetPaintColor))
  (Rendering|Material|SetVectorParameterValue (Variables|Default|GetDMI) "Color" (Variables|Default|GetPaintColor) :!class /Script/Engine.MaterialInstanceDynamic))

(fn ConstructionScript
  (|CallParentFunction))