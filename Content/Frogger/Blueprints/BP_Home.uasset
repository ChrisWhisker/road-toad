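; BP_Home is a goal home spot in the Frogger game, shown as a lily pad that can hold a frog.
; On BeginPlay it gives the lily pad a random yaw for visual variety.
; CloseHome shows the frog mesh and enables collision on a blocking box, while OpenHome hides the frog and disables that collision.
; The construction script starts the box with collision off.
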(event Custom|CloseHome
  (Collision|SetCollisionEnabled (Variables|Default|GetBlockingBox) "QueryAndPhysics")
  (Rendering|SetVisibility (Variables|Default|GetStaticMesh_Frog) true false))

(event Custom|OpenHome
  (Collision|SetCollisionEnabled (Variables|Default|GetBlockingBox) "NoCollision")
  (Rendering|SetVisibility (Variables|Default|GetStaticMesh_Frog) false false))

(event EventBeginPlay
  (|CallParentFunction)
  (Transformation|SetRelativeRotation (Variables|Default|GetStaticMesh_LilyPad) (Math|Rotator|MakeRotator 0.0 0.0 (Math|Random|RandomFloatinRange 0.0 3.6e+02)) false false))

(event Collision|EventActorBeginOverlap
  (params (OtherActor :type Actor%20Object%20Reference)))

(event EventTick
  (params (DeltaSeconds :type Float%20%28single-precision%29)))

(fn ConstructionScript
  (Collision|SetCollisionEnabled (Variables|Default|GetBlockingBox) "NoCollision"))