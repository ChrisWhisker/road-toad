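; BP_PowerUp is a Frogger power-up actor that can be switched on and off, with no pickup effect of its own.
; Enable and Disable toggle the mesh visibility and sphere collision together, and BeginPlay applies the initial Enabled state.
; Enabling also plays a timeline that animates the mesh scale as a multiple of the original scale cached at BeginPlay.
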(event Custom|Enable
  (Rendering|SetVisibility (Variables|Default|GetStaticMesh) true false)
  (Collision|SetCollisionEnabled (Variables|Default|GetSphere) "QueryAndPhysics")
  (Variables|Default|SetEnabled true)
  (bind _newtrack_0 (Timeline|Timeline_0 Play)
    (:Update
      (Transformation|SetRelativeScale3D (Variables|Default|GetStaticMesh) (* (Variables|Default|GetOriginalScale) _newtrack_0)))))

(event Custom|Disable
  (Rendering|SetVisibility (Variables|Default|GetStaticMesh) false false)
  (Collision|SetCollisionEnabled (Variables|Default|GetSphere) "NoCollision")
  (Variables|Default|SetEnabled false))

(event EventBeginPlay
  (Variables|Default|SetOriginalScale (Variables|/Script/Engine.SceneComponent|GetRelativeScale3D (Variables|Default|GetStaticMesh)))
  (if (Variables|Default|GetEnabled)
    (CallFunction|Enable)
    (else
      (Collision|SetCollisionEnabled (Variables|Default|GetSphere) "NoCollision")
      (Rendering|SetVisibility (Variables|Default|GetStaticMesh) false false))))

(fn ConstructionScript)